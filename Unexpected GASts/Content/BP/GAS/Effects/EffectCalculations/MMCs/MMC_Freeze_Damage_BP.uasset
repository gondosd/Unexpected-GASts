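; Gameplay Ability System magnitude calculation that sets freeze damage for a gameplay effect.
; It returns base damage at a fixed level, adding a captured attribute times a health-based freeze multiplier when the target is tagged Wet.
; Source and target tag containers are passed swapped into the attribute capture.
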(fn CalculateBaseMagnitude
  (params (Spec :type Gameplay%20Effect%20Spec%20Structure%20%28by%20ref%29))
  (bind _basedmg (Variables|Default|GetBaseDMG))
  (bind _returnvalue (Math|Conversions|ToFloat(Integer) _basedmg 1.0))
  (bind _returnvalue_2 (Class|GameplayModMagnitudeCalculation|GetSourceAggregatedTags Spec))
  (bind _returnvalue_3 (Class|GameplayModMagnitudeCalculation|GetTargetAggregatedTags Spec))
  (bind _returnvalue_4 (Class|GameplayModMagnitudeCalculation|GetCapturedAttributeMagnitude Spec "(AttributeName=\"Health\",Attribute=/Script/UnexpectedGASts.GD_AttributeSet:Health,AttributeOwner=\"/Script/CoreUObject.Class'/Script/UnexpectedGASts.GD_AttributeSet'\")" _returnvalue_3 _returnvalue_2))
  (if (GameplayTags|HasTag _returnvalue_3 "(TagName=\"GAS.Status.Wet\")")
    (return (+ (* _returnvalue_4 (Variables|Default|GetFreezeDMGMultiplierfromHealth)) _returnvalue))
    (else
      (return _returnvalue))))
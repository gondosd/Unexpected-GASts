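; Gameplay Ability that dashes the avatar character forward through pawns, damaging those it passes.
; On activation it commits the cooldown, sets the capsule to overlap pawns and applies a brief root motion force.
; Overlapped pawns receive GE_DashDamage at the ability's level, and ending the ability restores blocking and unbinds the overlap event.
; An unconnected alternative that dashes by a swept transform offset remains in the graph.
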(event Custom|Overlapped
  (params (OverlappedComponent :type Primitive%20Component%20Object%20Reference) (OtherActor :type Actor%20Object%20Reference) (OtherComp :type Primitive%20Component%20Object%20Reference) (OtherBodyIndex :type Integer) (bFromSweep :type Boolean) (SweepResult :type Hit%20Result%20Structure%20%28by%20ref%29))
  (bind _returnvalue (Ability|GetAbilitySystemComponentfromActorInfo))
  (Class|KismetSystemLibrary|IsObjectOfSoftClass OtherActor "/Script/Engine.Pawn"
    (:True
      (GameplayEffects|ApplyGameplayEffectSpecToTarget _returnvalue (GameplayEffects|MakeOutgoingSpec :self _returnvalue :GameplayEffectClass "/Game/BP/GAS/Effects/GE_DashDamage.GE_DashDamage_C" :Level (Math|Conversions|ToFloat(Integer) (Ability|GetAbilityLevel))) (Ability|GetAbilitySystemComponent OtherActor)))))

(event Ability|EventActivateAbility
  (Ability|CommitAbilityCooldown false)
  (bind _ascharacter (Utilities|Casting|CastToCharacter (Ability|GetAvatarActorfromActorInfo)))
  (bind _output_get (Variables|Default|SetAvatarCapsule (Variables|/Script/Engine.Character|GetCapsuleComponent _ascharacter)))
  (Collision|SetCollisionResponsetoChannel _output_get "ECC_Pawn" "ECR_Overlap")
  (Collision|BindEventtoOnComponentBeginOverlap (Variables|Default|GetAvatarCapsule) (EventDispatchers|CreateEvent :!event Custom|Overlapped))
  (Ability|Tasks|ApplyRootMotionConstantForce "None" (Math|Vector|GetForwardVector (Variables|Default|GetAvatarCapsule)) (Variables|Default|GetDash%20Strenght) 0.1 false 0 "MaintainLastRootMotionVelocity"
    (:OnFinish
      (Ability|EndAbility))))

(event Ability|EventOnEndAbility
  (params (bWasCancelled :type Boolean))
  (bind _avatarcapsule (Variables|Default|GetAvatarCapsule))
  (Collision|SetCollisionResponsetoChannel _avatarcapsule "ECC_Pawn" "ECR_Block")
  (EventDispatchers|UnbindallEventsfromOnComponentBeginOverlap _avatarcapsule))
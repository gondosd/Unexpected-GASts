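; GA_PrimaryAttack is a Gameplay Ability for the primary attack, a hitscan strike timed to an attack animation.
; Activation plays a montage picked by an attack-counter-seeded random stream, ending the ability when it completes or is cut short.
; In parallel it awaits the AttackNotify gameplay event, then traces forward from the avatar's spring arm socket.
; A hit actor with an ability system receives damage and freeze-stun effects and loses effects granting the Wet tag.
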(event Ability|EventOnEndAbility
  (params (bWasCancelled :type Boolean)))

(event Ability|EventActivateAbility
  (bind _returnvalue (Ability|GetAbilitySystemComponentfromActorInfo))
  (bind _returnvalue_2 (Ability|GetAvatarActorfromActorInfo))
  (bind _returnvalue_3 (Ability|GetAbilityLevel))
  (bind _returnvalue_4 (Actor|GetComponentsByClass _returnvalue_2 "/Script/Engine.SpringArmComponent"))
  (bind _returnvalue_5 (Math|Conversions|ToFloat(Integer) _returnvalue_3))
  (bind _output (Utilities|Array|Get(acopy) _returnvalue_4))
  (bind _returnvalue_6 (Transformation|GetSocketTransform _output "None" "RTS_World"))
  (Utilities|FlowControl|Sequence
    (:then_0
      (Math|Integer|IncrementInt (Variables|Default|GetAttackCounter)
        (:%20%20
          (|PlayMontageandWaitProxy "None" (.OutItem (Utilities|Array|RandomFromStream (Variables|Default|GetMontages%20to%20Play) (Math|Random|MakeRandomStream (* (Variables|Default|GetAttackCounter) 321)))) 1.0 "None" true 1.0 0.0 false
            (:OnCompleted
              _)
            (:OnInterrupted
              _)
            (:OnCancelled
              _))
          (Ability|EndAbility))))
    (:then_1
      (Ability|Tasks|WaitGameplayEvent "(TagName=\"GAS.Events.Attacks.AttackNotify\")" 0
        (:EventReceived
          (bind _outhit (Collision|LineTraceByChannel (.location _returnvalue_6) (+ (.location _returnvalue_6) (* (Math|Vector|GetForwardVector (.rotation _returnvalue_6)) 1e+04)) "TraceTypeQuery1" false (Utilities|Array|MakeArray (Ability|GetAvatarActorfromActorInfo)) "None"))
          (if (.bBlockingHit (Collision|BreakHitResult _outhit))
            (Utilities|IsValid (Ability|GetAbilitySystemComponent (.HitActor (Collision|BreakHitResult _outhit)))
              (:Is%20Valid
                (GameplayEffects|ApplyGameplayEffectToTarget :self _returnvalue :GameplayEffectClass "/Game/BP/GAS/Effects/GE_PrimaryDamage.GE_PrimaryDamage_C" :Target (Ability|GetAbilitySystemComponent (.HitActor (Collision|BreakHitResult _outhit))) :Level _returnvalue_5)
                (GameplayEffects|ApplyGameplayEffectToTarget :self _returnvalue :GameplayEffectClass "/Game/BP/GAS/Effects/GE_FreezeStun.GE_FreezeStun_C" :Target (Ability|GetAbilitySystemComponent (.HitActor (Collision|BreakHitResult _outhit))) :Level _returnvalue_5)
                (GameplayEffects|RemoveActiveEffectswithGrantedTags (Ability|GetAbilitySystemComponent (.HitActor (Collision|BreakHitResult _outhit))) "(GameplayTags=((TagName=\"GAS.Status.Wet\")))")))))))))
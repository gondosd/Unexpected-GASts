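; Fey character Blueprint that reacts to its death state through the Gameplay Ability System.
; On possession it binds a tag-changed event wrapper to GAS.States.Dead on its Ability System Component.
; While the tag is present it disables capsule collision and movement, and restores collision and walking when the tag clears.
; The logic is marked as a temporary way to see who died.
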(event Custom|CustomEvent
  (params (Tag :type Gameplay%20Tag%20Structure%20%28by%20ref%29) (TagCount :type Integer))
  ;[1 0 0 0.5] TEMP: so i can see who died
  (CallFunction|Change (> TagCount 0)))

(event Custom|Change
  (params (IsDead :type Boolean))
  ;[1 0 0 0.5] TEMP: so i can see who died
  (if IsDead
    (Collision|SetCollisionEnabled (Variables|Default|GetCapsuleComponent) "NoCollision")
    (Pawn|Components|CharacterMovement|DisableMovement (Variables|Character|GetCharacterMovement))
    (else
      (Collision|SetCollisionEnabled (Variables|Default|GetCapsuleComponent) "QueryAndPhysics")
      (Pawn|Components|CharacterMovement|SetMovementMode (Variables|Character|GetCharacterMovement) "MOVE_Walking" 0))))

(event EventPossessed
  (params (NewController :type Controller%20Object%20Reference))
  ;[1 0 0 0.5] TEMP: so i can see who died
  (GameplayTags|BindEventWrappertoGameplayTagChanged (Ability|GetAbilitySystemComponent 0) "(TagName=\"GAS.States.Dead\")" (delegate Custom|CustomEvent)))

(fn ConstructionScript)